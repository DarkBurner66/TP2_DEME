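; BP_Trap is a spike trap that fires when its slab is overlapped, once TrapActive has armed it.
; Two timelines drive the spike's relative Z, with a delay before the second lowers it and clears the SpikeActive re-trigger guard.
; A separate spike overlap applies negative HealthChangeAmount as damage to the ACHealth component on the third-person character's PlayerState, without checking trap state.
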(event `self.Slab collision.OnComponentBeginOverlap`
  (params (OverlappedComponent :type "PrimitiveComponent Object Reference") (OtherActor :type "Actor Object Reference") (OtherComp :type "PrimitiveComponent Object Reference") (OtherBodyIndex :type Integer) (bFromSweep :type Boolean) (SweepResult :type "HitResult Structure (by ref)"))
  (if (and (`self.Active`) (not (`self.SpikeActive`)))
    (set `self.SpikeActive` true)
    (bind (_direction _newtrack_2) (`Timeline|Timeline` :`NewTime` 2.0)
      (:`Update`
        (`SceneComponent.K2_SetRelativeLocation` (`self.Spike`) (`KismetMathLibrary.MakeVector` 0.0 0.0 (`KismetMathLibrary.Lerp` 0.0 0.0 _newtrack_2)) false false)
        (`KismetSystemLibrary.Delay` 2.0)
        (bind (_direction_2 _newtrack_2_2) (`Timeline|Timeline_0` :`NewTime` 2.0)
          (:`Update`
            (`SceneComponent.K2_SetRelativeLocation` (`self.Spike`) (`KismetMathLibrary.MakeVector` 0.0 0.0 (`KismetMathLibrary.Lerp` 0.0 -2.0 _newtrack_2_2)) false false)
            (set `self.SpikeActive` false)))))))

(event `self.SpikeDamage.OnComponentBeginOverlap`
  (params (OverlappedComponent :type "PrimitiveComponent Object Reference") (OtherActor :type "Actor Object Reference") (OtherComp :type "PrimitiveComponent Object Reference") (OtherBodyIndex :type Integer) (bFromSweep :type Boolean) (SweepResult :type "HitResult Structure (by ref)"))
  (bind _asbp_third_person_character (cast `/Game/Game/Blueprints/Pawns_Characters/Player/BP_ThirdPersonCharacter` OtherActor))
  (bind _output_get (set `self.As BP Third Person Character` _asbp_third_person_character))
  (bind _asbp_player_state (cast `/Game/Game/Blueprints/PlayerStates/BP_PlayerState` (`Pawn.PlayerState` _output_get)))
  (if (< (`self.HealthChangeAmount`) 0.0)
    (`/Game/Game/Blueprints/Components/AC_Health.TakeDamage` (`/Game/Game/Blueprints/PlayerStates/BP_PlayerState.AC_Health` _asbp_player_state) (`KismetMathLibrary.Abs` (`self.HealthChangeAmount`)))))

(event `/Game/Emile/Blueprints/BPI_TrapActivation.TrapActive`
  (`KismetSystemLibrary.PrintString` "Hello")
  (set `self.Active` true))

(fn `Activation`
  (returns (Interact :type Boolean))
  (return false))

(fn `UserConstructionScript`)