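; BP_GemPickup is a gem pickup that triggers traps when an actor overlaps it.
; On BeginPlay, one timeline drives the Diamond's yaw, and its update plays a second timeline that drives the Diamond's relative height.
; Any overlap, with no actor filter, sends TrapActiveMessage to every actor implementing BPI_TrapActivation.
; DestroyActor sits inside that loop, so the gem is destroyed only if at least one such actor exists.
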(event `self.ReceiveBeginPlay`
  (bind _diamond (`self.diamond`))
  (bind (_direction _nouvelle_piste_0) (`Timeline|Chronologie` :`NewTime` 2.0)
    (:`Update`
      (`SceneComponent.K2_SetRelativeRotation` _diamond (`KismetMathLibrary.MakeRotator` 0.0 0.0 (`KismetMathLibrary.Lerp` _nouvelle_piste_0 _nouvelle_piste_0)) false false)
      (bind (_direction_2 _nouvelle_piste_0_2) (`Timeline|Chronologie_0` :`NewTime` 2.0)
        (:`Update`
          (`SceneComponent.K2_SetRelativeLocation` _diamond (`KismetMathLibrary.MakeVector` 0.0 0.0 (`KismetMathLibrary.Lerp` _nouvelle_piste_0_2 _nouvelle_piste_0_2)) false false))))))

(event `self.ReceiveActorBeginOverlap`
  (params (OtherActor :type "Actor Object Reference"))
  (bind _outactors (`GameplayStatics.GetAllActorsWithInterface` "/Game/Emile/Blueprints/BPI_TrapActivation.BPI_TrapActivation_C"))
  (for _array_element _outactors
    (message `/Game/Emile/Blueprints/BPI_TrapActivation.TrapActive` _array_element)
    (`self.K2_DestroyActor`)))

(fn `UserConstructionScript`)