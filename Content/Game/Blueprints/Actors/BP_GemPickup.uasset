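; Gem pickup actor that animates its diamond mesh with timelines and, when interacted with, triggers the level's traps and destroys itself.
; The construction script configures mesh and sphere trigger from variables, though SetupUI repositions the Diamond rather than InteractUI.
; Trigger begin overlap registers it with BP_ThirdPersonCharacter, while InteractUI end overlap unregisters it.
; Interact messages BPI_TrapActivation actors, calling DestroyActor inside that loop.
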(event `self.ReceiveBeginPlay`
  ; Gérer l'animation de la gemme
  (bind (_direction _newtrack_0) (`Timeline|Timeline` :`NewTime` 2.0)
    (:`Update`
      (`SceneComponent.K2_SetRelativeRotation` (`self.diamond`) (`KismetMathLibrary.MakeRotator` 0.0 0.0 (`KismetMathLibrary.Lerp` _newtrack_0 360.0)) false false)
      (bind (_direction_2 _newtrack_0_2) (`Timeline|Timeline_0` :`NewTime` 2.0)
        (:`Update`
          (`SceneComponent.K2_SetRelativeLocation` (`self.diamond`) (`KismetMathLibrary.MakeVector` 0.0 0.0 (`KismetMathLibrary.Lerp` _newtrack_0_2 2.0)) false false))))))

(event `self.InteractTrigger.OnComponentBeginOverlap`
  (params (OverlappedComponent :type "PrimitiveComponent Object Reference") (OtherActor :type "Actor Object Reference") (OtherComp :type "PrimitiveComponent Object Reference") (OtherBodyIndex :type Integer) (bFromSweep :type Boolean) (SweepResult :type "HitResult Structure (by ref)"))
  ; Interaction trigger qui active l'interaction lorsqu'on overlap avec la gemme
  (bind _asbp_third_person_character (cast `/Game/Game/Blueprints/Pawns_Characters/Player/BP_ThirdPersonCharacter` OtherActor))
  (`/Game/Game/Blueprints/Pawns_Characters/Player/BP_ThirdPersonCharacter.AddInteractionDiamond` _asbp_third_person_character self))

(event `self.InteractUI.OnComponentEndOverlap`
  (params (OverlappedComponent :type "PrimitiveComponent Object Reference") (OtherActor :type "Actor Object Reference") (OtherComp :type "PrimitiveComponent Object Reference") (OtherBodyIndex :type Integer))
  ; Interaction trigger qui active l'interaction lorsqu'on overlap avec la gemme
  (bind _asbp_third_person_character (cast `/Game/Game/Blueprints/Pawns_Characters/Player/BP_ThirdPersonCharacter` OtherActor))
  (`/Game/Game/Blueprints/Pawns_Characters/Player/BP_ThirdPersonCharacter.RemoveInteractionDiamond` _asbp_third_person_character self))

(event `TrapActivated`
  ; Activation des traps
  (bind _outactors (`GameplayStatics.GetAllActorsWithInterface` "/Game/Game/Blueprints/Interfaces/BPI_TrapActivation.BPI_TrapActivation_C"))
  (for _array_element _outactors
    (message `/Game/Game/Blueprints/Interfaces/BPI_TrapActivation.TrapActive` _array_element)
    (`self.K2_DestroyActor`)))

(fn `Interact`
  (params (Interact :type "/Game/Game/Blueprints/Pawns_Characters/Player/BP_ThirdPersonCharacter Object Reference"))
  ; Lorsque l'interaction est activé, il active le blueprint TrapActivated
  (set `self.Interact Character` Interact)
  (`self.TrapActivated`))

(fn `SetupMesh`
  ; Setup Mesh
  (`StaticMeshComponent.SetStaticMesh` (`self.diamond`) (`self.InteractionMesh`))
  (`SceneComponent.K2_SetRelativeTransform` (`self.diamond`) (`self.MeshTransform`) false false))

(fn `SetupTrigger`
  ; Setup Trigger
  (`SphereComponent.SetSphereRadius` (`self.InteractTrigger`) (`self.TriggerRadius`) true)
  (`SceneComponent.K2_SetRelativeLocation` (`self.InteractTrigger`) (`self.TriggerLocation`) false false))

(fn `SetupUI`
  ; Setup UI
  (`SceneComponent.K2_SetRelativeLocation` (`self.diamond`) (`self.UI_Location`) false false))

(fn `ToggleUI`
  (params (Visible :type Boolean))
  ; Toggle UI
  (`SceneComponent.SetVisibility` (`self.InteractUI`) Visible false))

(fn `UserConstructionScript`
  (`self.SetupMesh`)
  (`self.SetupTrigger`)
  (`self.SetupUI`))