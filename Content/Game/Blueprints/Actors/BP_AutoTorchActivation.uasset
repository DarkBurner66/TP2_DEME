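; BP_AutoTorchActivation is an actor that automatically lights an array of BP_Torch actors when play begins.
; On BeginPlay it steps through the Torches array by index, casting each entry to BP_Torch and calling StartFire, with a 0.1-second Delay loop staggering the ignitions.
; The inclusive length check runs one index past the end, so the loop ends on a failed cast, as it does at any invalid entry.
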(event `self.ReceiveBeginPlay`
  ; Allume tous les BP_Torche dans le tableau dès que le niveau est chargé
  (bind _asbp_torch (cast `/Game/Game/Blueprints/Actors/BP_Torch` (`|GetArrayItem` (`self.Torches`) (`self.Torche Number`)) :!label _label))
  (`/Game/Game/Blueprints/Actors/BP_Torch.Start Fire` _asbp_torch)
  (set `self.Torche Number` (+ (`self.Torche Number`) 1))
  (if (<= (`self.Torche Number`) (`KismetArrayLibrary.Array_Length` (`self.Torches`)))
    (`KismetSystemLibrary.Delay` 0.1)
    (goto _label)))

(fn `UserConstructionScript`)