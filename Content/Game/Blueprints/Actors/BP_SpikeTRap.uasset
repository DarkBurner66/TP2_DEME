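; BP_SpikeTRap is a one-shot spike trap that kills the player character on contact and leads to the losing screen.
; Overlapping TrapTrigger plays a sound, then after a delay timelines slide the spikes along local Y and, following another delay, back, destroying the trigger.
; Overlapping DamageTrigger sends damage to the PlayerState's health component, shows hurt and death widgets, then loads the MenuFin_Perdant level instance after a delay.
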(event `self.TrapTrigger.OnComponentBeginOverlap`
  (params (OverlappedComponent :type "PrimitiveComponent Object Reference") (OtherActor :type "Actor Object Reference") (OtherComp :type "PrimitiveComponent Object Reference") (OtherBodyIndex :type Integer) (bFromSweep :type Boolean) (SweepResult :type "HitResult Structure (by ref)"))
  ; Trap activation
  (cast `/Game/Game/Blueprints/Pawns_Characters/Player/BP_ThirdPersonCharacter` OtherActor)
  (`GameplayStatics.PlaySoundAtLocation` "/Game/Game/Audio/SFX/Trap/S_trap_Cue.S_trap_Cue" (`SceneComponent.K2_GetComponentLocation` (`self.spike_trap`)) (struct) 1.0 1.0 0.0 null null null null)
  (`KismetSystemLibrary.Delay` 2.0)
  (bind (_direction _alpha) (`Timeline|SpikeTrap forward`)
    (:`Update`
      (`SceneComponent.K2_SetRelativeLocation` (`self.spike_trap`) (`KismetMathLibrary.MakeVector` 0.0 (`KismetMathLibrary.Lerp` 0.0 325.0 _alpha)) false false)
      ; trap back
      (`KismetSystemLibrary.Delay` 2.0)
      (bind (_direction_2 _alpha_2) (`Timeline|SpikeTrap back`)
        (:`Update`
          (`SceneComponent.K2_SetRelativeLocation` (`self.spike_trap`) (`KismetMathLibrary.MakeVector` 0.0 (`KismetMathLibrary.Lerp` 0.0 325.0 _alpha_2)) false false)
          ; trap deactivate
          (`ActorComponent.K2_DestroyComponent` (`self.TrapTrigger`)))))))

(event `self.DamageTrigger.OnComponentBeginOverlap`
  (params (OverlappedComponent :type "PrimitiveComponent Object Reference") (OtherActor :type "Actor Object Reference") (OtherComp :type "PrimitiveComponent Object Reference") (OtherBodyIndex :type Integer) (bFromSweep :type Boolean) (SweepResult :type "HitResult Structure (by ref)"))
  ; Death
  (bind _asbp_third_person_character (cast `/Game/Game/Blueprints/Pawns_Characters/Player/BP_ThirdPersonCharacter` OtherActor))
  (bind _output_get (set `self.As BP Third Person Character` _asbp_third_person_character))
  (bind _asbp_player_state (cast `/Game/Game/Blueprints/PlayerStates/BP_PlayerState` (`Pawn.PlayerState` _output_get)))
  (message `/Game/Game/Blueprints/Interfaces/BPI_Damageable.TakeDamage` (`/Game/Game/Blueprints/PlayerStates/BP_PlayerState.AC_Health` _asbp_player_state) (`KismetMathLibrary.Abs` (`self.Death`)))
  (bind _returnvalue (`|CreateWidget` "/Game/Game/UI/WBP_Hurt.WBP_Hurt_C"))
  (`UserWidget.AddToViewport` _returnvalue 0)
  (bind _returnvalue_2 (`|CreateWidget` "/Game/Emile/UI/BP_Died.BP_Died_C"))
  (`UserWidget.AddToViewport` _returnvalue_2 0)
  (`KismetSystemLibrary.Delay` 2.0)
  (`LevelStreamingDynamic.LoadLevelInstance` " MenuFin_Perdant" (0.0 0.0 0.0) (struct) "" null))

(fn `UserConstructionScript`)