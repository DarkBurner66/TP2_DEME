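; BP_Interact_Chest is an interactable chest actor with a mesh, a trigger sphere and an interaction UI component.
; The construction script applies its variables to set the mesh and transform, the trigger radius and location, and the UI location.
; Trigger overlaps call AddInteraction and RemoveInteraction on BP_ThirdPersonCharacter.
; ToggleUI sets prompt visibility, and Interact only stores the interacting character, with no opening logic here.
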(event `self.InteractTrigger.OnComponentBeginOverlap`
  (params (OverlappedComponent :type "PrimitiveComponent Object Reference") (OtherActor :type "Actor Object Reference") (OtherComp :type "PrimitiveComponent Object Reference") (OtherBodyIndex :type Integer) (bFromSweep :type Boolean) (SweepResult :type "HitResult Structure (by ref)"))
  ; Trigger overlap
  (bind _asbp_third_person_character (cast `/Game/Game/Blueprints/Pawns_Characters/Player/BP_ThirdPersonCharacter` OtherActor))
  (`/Game/Game/Blueprints/Pawns_Characters/Player/BP_ThirdPersonCharacter.AddInteraction` _asbp_third_person_character null))

(event `self.InteractTrigger.OnComponentEndOverlap`
  (params (OverlappedComponent :type "PrimitiveComponent Object Reference") (OtherActor :type "Actor Object Reference") (OtherComp :type "PrimitiveComponent Object Reference") (OtherBodyIndex :type Integer))
  ; Trigger overlap
  (bind _asbp_third_person_character (cast `/Game/Game/Blueprints/Pawns_Characters/Player/BP_ThirdPersonCharacter` OtherActor))
  (`/Game/Game/Blueprints/Pawns_Characters/Player/BP_ThirdPersonCharacter.RemoveInteraction` _asbp_third_person_character null))

(fn `Interact`
  (params (Character :type "/Game/Game/Blueprints/Pawns_Characters/Player/BP_ThirdPersonCharacter Object Reference"))
  ; Interact
  (set `self.Interact Character` Character))

(fn `SetupMesh`
  ; SetupMesh
  (`StaticMeshComponent.SetStaticMesh` (`self.InteractMesh`) (`self.InteractionMesh`))
  (`SceneComponent.K2_SetRelativeTransform` (`self.InteractMesh`) (`self.MeshTansform`) false false))

(fn `SetupTrigger`
  ; Trigger setup
  (`SphereComponent.SetSphereRadius` (`self.InteractTrigger`) (`self.TriggerRadius`) true)
  (`SceneComponent.K2_SetRelativeLocation` (`self.InteractTrigger`) (`self.TriggerLocation`) false false))

(fn `SetupUI`
  ; Setup UI
  (`SceneComponent.K2_SetRelativeLocation` (`self.InteractUI`) (`self.UI_Location`) false false))

(fn `ToggleUI`
  (params (Visible :type Boolean))
  ; set visibility
  (`SceneComponent.SetVisibility` (`self.InteractUI`) Visible false))

(fn `UserConstructionScript`
  (`self.SetupMesh`)
  (`self.SetupTrigger`)
  (`self.SetupUI`))