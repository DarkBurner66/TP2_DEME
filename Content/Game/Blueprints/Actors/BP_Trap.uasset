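; BP_Trap is a floor spike trap that hurts the player character and stays inert until the TrapActive interface event arms it.
; Stepping on the slab while armed plays a sound and two delay-separated timelines that move the spike, with SpikeActive guarding against retriggering.
; A separate SpikeDamage overlap applies negative HealthChangeAmount as damage through the PlayerState's health component, without checking whether the trap is armed.
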(event `self.Slab collision.OnComponentBeginOverlap`
  (params (OverlappedComponent :type "PrimitiveComponent Object Reference") (OtherActor :type "Actor Object Reference") (OtherComp :type "PrimitiveComponent Object Reference") (OtherBodyIndex :type Integer) (bFromSweep :type Boolean) (SweepResult :type "HitResult Structure (by ref)"))
  ; Lorsqu'on collide avec un trap, si ''Active'' est égal a true et que ''spike active'' est égal a false: On met spike active a true et on joue l'animation du spike. Après l'animation, on remet ''spike active'' a false, afin de ne pas recommencer l'animation si on overlapp quand l'animation joue déja.
  (cast `/Game/Game/Blueprints/Pawns_Characters/Player/BP_ThirdPersonCharacter` OtherActor)
  (if (and (`self.Active`) (not (`self.SpikeActive`)))
    (`GameplayStatics.PlaySound2D` "/Game/Game/Audio/SFX/SpikeTrap.SpikeTrap" 1.0 1.0 0.0 null null)
    (set `self.SpikeActive` true)
    (bind (_direction _newtrack_2) (`Timeline|Timeline` :`NewTime` 2.0)
      (:`Update`
        (`SceneComponent.K2_SetRelativeLocation` (`self.Spike`) (`KismetMathLibrary.MakeVector` 0.0 0.0 (`KismetMathLibrary.Lerp` 0.0 0.0 _newtrack_2)) false false)
        (`KismetSystemLibrary.Delay` 2.0)
        (bind (_direction_2 _newtrack_2_2) (`Timeline|Timeline_0` :`NewTime` 2.0)
          (:`Update`
            (`SceneComponent.K2_SetRelativeLocation` (`self.Spike`) (`KismetMathLibrary.MakeVector` 0.0 0.0 (`KismetMathLibrary.Lerp` 0.0 -2.0 _newtrack_2_2)) false false)
            (set `self.SpikeActive` false)))))))

(event `self.SpikeDamage.OnComponentBeginOverlap`
  (params (OverlappedComponent :type "PrimitiveComponent Object Reference") (OtherActor :type "Actor Object Reference") (OtherComp :type "PrimitiveComponent Object Reference") (OtherBodyIndex :type Integer) (bFromSweep :type Boolean) (SweepResult :type "HitResult Structure (by ref)"))
  ; De plus, lorsque le joueur overlap avec le trap Actif, il fait des dommage au joueur.
  (bind _asbp_third_person_character (cast `/Game/Game/Blueprints/Pawns_Characters/Player/BP_ThirdPersonCharacter` OtherActor))
  (bind _output_get (set `self.As BP Third Person Character` _asbp_third_person_character))
  (bind _asbp_player_state (cast `/Game/Game/Blueprints/PlayerStates/BP_PlayerState` (`Pawn.PlayerState` _output_get)))
  (if (< (`self.HealthChangeAmount`) 0.0)
    (`/Game/Game/Blueprints/Components/AC_Health.TakeDamage` (`/Game/Game/Blueprints/PlayerStates/BP_PlayerState.AC_Health` _asbp_player_state) (`KismetMathLibrary.Abs` (`self.HealthChangeAmount`)))))

(event `/Game/Game/Blueprints/Interfaces/BPI_TrapActivation.TrapActive`
  ; Lorsque le blueprint interface ''TrapActive'' est activé, on met le boolean ''Active'' a ''true''
  (`KismetSystemLibrary.PrintString` "Hello")
  (set `self.Active` true))

(fn `Activation`
  (returns (Interact :type Boolean))
  (return false))

(fn `UserConstructionScript`)