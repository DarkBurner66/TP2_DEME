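; Health component that tracks current health, handles damage, healing and reset, and drives the death sequence.
; All changes go through UpdateHealthAndNotify, which clamps the value and broadcasts OnHealthChanged to listeners.
; Damage plays a hurt sound, and both damage and healing are ignored once dead.
; At zero health it fires OnDeath, plays a death sound, shows the death widget and calls LoadLevel on the third-person game mode.
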(event `/Game/Game/Blueprints/Interfaces/BPI_Damageable.TakeDamage`
  (params (DamageAmount :type "Float (double-precision)"))
  ; Lorsque le personnage prend du dégat, il fait un son de douleur
  (if (not (`self.IsDead`))
    (`GameplayStatics.PlaySound2D` "/Game/Game/Audio/SFX/Grunt/S_Hurt_Cue.S_Hurt_Cue" 1.0 1.0 0.0 null null)
    (`self.UpdateHealthAndNotify` (- (`self.CurrentHealth`) DamageAmount))
    (`KismetSystemLibrary.PrintString` (`KismetStringLibrary.Conv_DoubleToString` (`self.CurrentHealth`)))))

(event `/Game/Game/Blueprints/Interfaces/BPI_Damageable.GainHealth`
  (params (HealthAmount :type "Float (double-precision)"))
  (if (not (`self.IsDead`))
    (`self.UpdateHealthAndNotify` (+ (`self.CurrentHealth`) HealthAmount))
    (`KismetSystemLibrary.PrintString` (`KismetStringLibrary.Conv_DoubleToString` (`self.CurrentHealth`)))))

(event `/Game/Game/Blueprints/Interfaces/BPI_Damageable.ResetHealth`
  (set `self.IsDead` false)
  (`self.UpdateHealthAndNotify` (`self.MaxHealth`)))

(fn `UpdateHealthAndNotify`
  (params (NewHealthValue :type "Float (double-precision)"))
  (bind _maxhealth (`self.MaxHealth`))
  ; Mise à jour des variables de vie dans le AC_Health et call event OnHealthChanged pour notifié les listener d'un changement de vie et event OnDead si vie à 0 et joue un son en plus d'ajouter le widget de mort
  (bind _output_get (set `self.CurrentHealth` (`KismetMathLibrary.FClamp` NewHealthValue 0.0 _maxhealth)))
  (`self.OnHealthChanged` _output_get _maxhealth)
  (if (<= (`self.CurrentHealth`) 0.0)
    (set `self.IsDead` true)
    (`self.OnDeath`)
    (`GameplayStatics.PlaySound2D` "/Game/Game/Audio/SFX/Death/S_Death_Cue.S_Death_Cue" 1.0 1.0 0.0 null null)
    (bind _returnvalue (`|CreateWidget` "/Game/Emile/UI/BP_Died.BP_Died_C"))
    (`UserWidget.AddToViewport` _returnvalue 0)
    (bind _asbp_third_person_game_mode (cast `/Game/Game/Blueprints/GameModes/BP_ThirdPersonGameMode` (`GameplayStatics.GetGameMode`)))
    (`/Game/Game/Blueprints/GameModes/BP_ThirdPersonGameMode.LoadLevel` _asbp_third_person_game_mode)
    (else
      (set `self.IsDead` false))))