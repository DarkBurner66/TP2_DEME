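; Player state that owns the player's health component, keeps its values persistent through BP_GameInstance and handles death.
; On BeginPlay it restores saved health from the game instance, or resets health and sets the init flag on first use.
; Every health change writes current and max health back to the game instance.
; On death it plays a sound, shows the BP_Died widget and asks BP_ThirdPersonGameMode to start respawn.
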(event `self.ReceiveBeginPlay`
  (bind _asbp_game_instance (cast `/Game/Game/Blueprints/BP_GameInstance` (`GameplayStatics.GetGameInstance`)))
  (bind _output_get (set `self.RefGameInstance` _asbp_game_instance))
  (if (`/Game/Game/Blueprints/BP_GameInstance.HealthInit_GI` _output_get)
    (`self.LoadHealthFromGameInstance`)
    (else
      (`/Game/Game/Blueprints/Components/AC_Health.ResetHealth` (`self.AC_Health`))
      (set `/Game/Game/Blueprints/BP_GameInstance.HealthInit_GI` true _output_get))))

(event `self.AC_Health.OnDeath`
  (bind _asbp_third_person_game_mode (cast `/Game/Game/Blueprints/GameModes/BP_ThirdPersonGameMode` (`GameplayStatics.GetGameMode`)))
  (`GameplayStatics.PlaySound2D` "/Game/Game/Audio/SFX/Death/S_Death_Cue.S_Death_Cue" 1.0 1.0 0.0 null null)
  (bind _returnvalue (`|CreateWidget` "/Game/Emile/UI/BP_Died.BP_Died_C"))
  (`UserWidget.AddToViewport` _returnvalue 0)
  (`/Game/Game/Blueprints/GameModes/BP_ThirdPersonGameMode.StartRespawn` _asbp_third_person_game_mode (`GameplayStatics.GetPlayerController` 0)))

(event `self.AC_Health.OnHealthChanged`
  (params (CurrentHealth :type "Float (double-precision)") (MaxHealth :type "Float (double-precision)"))
  (`|ExecutionSequence`
    (:`then_0`
      (`self.SaveCurrentHealth` CurrentHealth))
    (:`then_1`
      (`self.SaveMaxHealth` MaxHealth))))

(fn `LoadHealthFromGameInstance`
  (bind _refgameinstance (`self.RefGameInstance`))
  (bind _ac_health (`self.AC_Health`))
  (bind _output_get (set `/Game/Game/Blueprints/Components/AC_Health.MaxHealth` (`/Game/Game/Blueprints/BP_GameInstance.MaxHealth_GI` _refgameinstance) _ac_health))
  (bind _output_get_2 (set `/Game/Game/Blueprints/Components/AC_Health.CurrentHealth` (`/Game/Game/Blueprints/BP_GameInstance.CurrentHealth_GI` _refgameinstance) _ac_health))
  (`/Game/Game/Blueprints/Components/AC_Health.OnHealthChanged` (`self.AC_Health`) _output_get_2 _output_get))

(fn `SaveCurrentHealth`
  (params (NewHealth :type "Float (double-precision)"))
  (set `/Game/Game/Blueprints/BP_GameInstance.CurrentHealth_GI` NewHealth (`self.RefGameInstance`)))

(fn `SaveMaxHealth`
  (params (NewMaxHealth :type "Float (double-precision)"))
  (set `/Game/Game/Blueprints/BP_GameInstance.MaxHealth_GI` NewMaxHealth (`self.RefGameInstance`)))

(fn `UserConstructionScript`)